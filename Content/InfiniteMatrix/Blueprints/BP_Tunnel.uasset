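; BP_Tunnel is an endless-runner tunnel segment with a rotating holed wall, health pack and bomb.
; The trigger zone requests the next tunnel, destroys this one, and raises player score and clamped speed.
; Hitting the wall costs score and registers a hit; pickup and bomb overlaps adjust health, while projectiles score by displacing the bomb.
; Randomize functions, not called here, vary wall shape, roll and item placement.
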(event OnComponentBeginOverlap(Bomb)
  (params (OverlappedComponent :type Primitive%20Component%20Object%20Reference) (OtherActor :type Actor%20Object%20Reference) (OtherComp :type Primitive%20Component%20Object%20Reference) (OtherBodyIndex :type Integer) (bFromSweep :type Boolean) (SweepResult :type Hit%20Result%20Structure%20%28by%20ref%29)))

(event OnComponentBeginOverlap(Healthpack)
  (params (OverlappedComponent :type Primitive%20Component%20Object%20Reference) (OtherActor :type Actor%20Object%20Reference) (OtherComp :type Primitive%20Component%20Object%20Reference) (OtherBodyIndex :type Integer) (bFromSweep :type Boolean) (SweepResult :type Hit%20Result%20Structure%20%28by%20ref%29))
  (bind _asbp_player (Utilities|Casting|CastToBP_Player OtherActor))
  (bind _output_get (Variables|/Game/InfiniteMatrix/Blueprints/BP_Player.BP_Player_C|SetCurrentHealth _asbp_player (Math|Float|Clamp(Float) (+ (Variables|/Game/InfiniteMatrix/Blueprints/BP_Player.BP_Player_C|GetCurrentHealth _asbp_player) (Variables|Default|GetHeal)) 0.0 (Variables|/Game/InfiniteMatrix/Blueprints/BP_Player.BP_Player_C|GetMaxHealth _asbp_player))))
  (Default|UpdateHealthUI (Variables|/Game/InfiniteMatrix/Blueprints/BP_Player.BP_Player_C|GetHealthBar _asbp_player) _output_get (Variables|/Game/InfiniteMatrix/Blueprints/BP_Player.BP_Player_C|GetMaxHealth _asbp_player)))

(event OnComponentBeginOverlap(WallMesh)
  (params (OverlappedComponent :type Primitive%20Component%20Object%20Reference) (OtherActor :type Actor%20Object%20Reference) (OtherComp :type Primitive%20Component%20Object%20Reference) (OtherBodyIndex :type Integer) (bFromSweep :type Boolean) (SweepResult :type Hit%20Result%20Structure%20%28by%20ref%29))
  (bind _asbp_player (Utilities|Casting|CastToBP_Player OtherActor))
  (bind _output_get (Variables|/Game/InfiniteMatrix/Blueprints/BP_Player.BP_Player_C|SetScore _asbp_player (- (Variables|/Game/InfiniteMatrix/Blueprints/BP_Player.BP_Player_C|GetScore _asbp_player) (Variables|Default|GetPlusScore))))
  (Default|UpdateScoreUI (Variables|/Game/InfiniteMatrix/Blueprints/BP_Player.BP_Player_C|GetScoreUI _asbp_player) _output_get)
  (Default|ProcessHit _asbp_player)
  (if (Variables|/Game/InfiniteMatrix/Blueprints/BP_Player.BP_Player_C|GetIsDead _asbp_player)
    (Default|DisplayRestart _asbp_player)))

(event OnComponentBeginOverlap(TriggerZone)
  (params (OverlappedComponent :type Primitive%20Component%20Object%20Reference) (OtherActor :type Actor%20Object%20Reference) (OtherComp :type Primitive%20Component%20Object%20Reference) (OtherBodyIndex :type Integer) (bFromSweep :type Boolean) (SweepResult :type Hit%20Result%20Structure%20%28by%20ref%29))
  (bind _asbp_player (Utilities|Casting|CastToBP_Player OtherActor))
  (Default|SpawnTunnelatSpawnPoint (Variables|Default|GetTunnelSpawner))
  (Actor|DestroyActor)
  (Default|UpdateScoreUI (Variables|/Game/InfiniteMatrix/Blueprints/BP_Player.BP_Player_C|GetScoreUI _asbp_player) (+ (Variables|/Game/InfiniteMatrix/Blueprints/BP_Player.BP_Player_C|GetScore _asbp_player) (Variables|Default|GetPlusScore)))
  (Variables|/Game/InfiniteMatrix/Blueprints/BP_Player.BP_Player_C|SetScore _asbp_player (+ (Variables|/Game/InfiniteMatrix/Blueprints/BP_Player.BP_Player_C|GetScore _asbp_player) (Variables|Default|GetPlusScore)))
  (Variables|/Game/InfiniteMatrix/Blueprints/BP_Player.BP_Player_C|SetForwardSpeed _asbp_player (Math|Float|Clamp(Float) (+ (Variables|/Game/InfiniteMatrix/Blueprints/BP_Player.BP_Player_C|GetForwardSpeed _asbp_player) (Variables|Default|GetAddSpeed)) 2e+03 4e+03)))

(event OnComponentEndOverlap(Bomb)
  (params (OverlappedComponent :type Primitive%20Component%20Object%20Reference) (OtherActor :type Actor%20Object%20Reference) (OtherComp :type Primitive%20Component%20Object%20Reference) (OtherBodyIndex :type Integer))
  (bind _asbp_player (Utilities|Casting|CastToBP_Player OtherActor)
    (:then
      (bind _output_get (Variables|/Game/InfiniteMatrix/Blueprints/BP_Player.BP_Player_C|SetCurrentHealth _asbp_player (Math|Float|Clamp(Float) (- (Variables|/Game/InfiniteMatrix/Blueprints/BP_Player.BP_Player_C|GetCurrentHealth _asbp_player) 5.0) 0.0 (Variables|/Game/InfiniteMatrix/Blueprints/BP_Player.BP_Player_C|GetMaxHealth _asbp_player))))
      (Default|UpdateHealthUI (Variables|/Game/InfiniteMatrix/Blueprints/BP_Player.BP_Player_C|GetHealthBar _asbp_player) _output_get (Variables|/Game/InfiniteMatrix/Blueprints/BP_Player.BP_Player_C|GetMaxHealth _asbp_player)))
    (:CastFailed
      (bind _asbp_projectile (Utilities|Casting|CastToBP_Projectile OtherActor))
      (bind _output_get_2 (Variables|/Game/InfiniteMatrix/Blueprints/BP_Player.BP_Player_C|SetScore (Variables|/Game/InfiniteMatrix/Blueprints/BP_Projectile.BP_Projectile_C|Getbpplayer _asbp_projectile) (+ (Variables|/Game/InfiniteMatrix/Blueprints/BP_Player.BP_Player_C|GetScore (Variables|/Game/InfiniteMatrix/Blueprints/BP_Projectile.BP_Projectile_C|Getbpplayer _asbp_projectile)) (Variables|Default|GetDestroyBomb))))
      (Default|UpdateScoreUI (Variables|/Game/InfiniteMatrix/Blueprints/BP_Player.BP_Player_C|GetScoreUI (Variables|/Game/InfiniteMatrix/Blueprints/BP_Projectile.BP_Projectile_C|Getbpplayer _asbp_projectile)) _output_get_2)
      (Transformation|SetRelativeLocation (Variables|Default|GetBomb) "0.000000,8000.000000,0.000000" false false))))

(event EventBeginPlay)

(event EventTick
  (params (DeltaSeconds :type Float%20%28single-precision%29))
  (Transformation|AddLocalRotation (Variables|Default|GetWallMesh) (Math|Rotator|MakeRotator (* DeltaSeconds (Variables|Default|GetRotateSpeed)) 0.0 0.0) false false))

(fn ConstructionScript)

(fn RandomizeWall
  (Components|StaticMesh|SetStaticMesh (Variables|Default|GetWallMesh) (Utilities|Select :Index (Math|Random|RandomIntegerinRange 0 3) :Option%200 "/Game/InfiniteMatrix/Meshes/SM_Hole_01.SM_Hole_01" :Option%201 "/Game/InfiniteMatrix/Meshes/SM_Hole_02.SM_Hole_02" :Option%202 "/Game/InfiniteMatrix/Meshes/SM_Hole_03.SM_Hole_03" :Option%203 "/Game/InfiniteMatrix/Meshes/SM_Hole_04.SM_Hole_04"))
  (Transformation|AddLocalRotation (Variables|Default|GetWallMesh) (Math|Rotator|MakeRotator (Math|Random|RandomFloatinRange 0.0 3.6e+02) 0.0 0.0) false false))

(fn RandomizeHealthPack
  (if (< (Math|Random|RandomIntegerinRange 0 3) 1)
    (Components|StaticMesh|SetStaticMesh (Variables|Default|GetHealthpack) "/Game/InfiniteMatrix/Meshes/Healthpack.Healthpack")
    (Transformation|SetRelativeLocation (Variables|Default|GetHealthpack) (Math|Vector|MakeVector (Math|Random|RandomFloatinRange 8e+02 1.8e+03) (Math|Random|RandomFloatinRange -3e+02 3e+02) (Math|Random|RandomFloatinRange -5e+02 -9e+02)) false false)))

(fn RandomizeBomb
  (bind _bomb (Variables|Default|GetBomb))
  (Components|StaticMesh|SetStaticMesh _bomb "/Game/InfiniteMatrix/Meshes/Bomb.Bomb")
  (Transformation|SetRelativeLocation _bomb (Math|Vector|MakeVector 1.8e+03 0.0 (Math|Float|SelectFloat -2e+02 1e+02 (> (Math|Random|RandomInteger 2) 0))) false false))